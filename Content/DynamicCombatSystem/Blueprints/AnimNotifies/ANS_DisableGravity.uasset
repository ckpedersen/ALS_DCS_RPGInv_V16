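; Anim notify state that suspends gravity on the owning Character for the span of an animation window.
; On begin it stops movement immediately and zeroes the CharacterMovement gravity scale.
; On end it stops movement again and sets gravity scale back to a fixed default of one rather than restoring the previous value.
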(fn `Received_NotifyBegin`
  (params (MeshComp :type "SkeletalMeshComponent Object Reference") (Animation :type "AnimSequenceBase Object Reference") (TotalDuration :type "Float (double-precision)"))
  (returns (ReturnValue :type Boolean))
  (bind _charactermovement (`Character.CharacterMovement` (cast `Character` (`ActorComponent.GetOwner` MeshComp) :!pure true)))
  (`MovementComponent.StopMovementImmediately` _charactermovement)
  (set `CharacterMovementComponent.GravityScale` 0.0 _charactermovement)
  (return false))

(fn `Received_NotifyEnd`
  (params (MeshComp :type "SkeletalMeshComponent Object Reference") (Animation :type "AnimSequenceBase Object Reference"))
  (returns (ReturnValue :type Boolean))
  (bind _charactermovement (`Character.CharacterMovement` (cast `Character` (`ActorComponent.GetOwner` MeshComp) :!pure true)))
  (`MovementComponent.StopMovementImmediately` _charactermovement)
  (set `CharacterMovementComponent.GravityScale` 1.0 _charactermovement)
  (return false))