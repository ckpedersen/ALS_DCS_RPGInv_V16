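; An animation notify that repositions and shows or hides the bow arrow on a combat character during archery animations.
; It casts the mesh owner to BP_CombatCharacter, then snaps the BowArrow component either to the character mesh at its bow-string socket or to the bow mesh's arrow socket, depending on AttachToHand.
; It finally sets the arrow's visibility from the ArrowVisibility setting.
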(fn `Received_Notify`
  (params (MeshComp :type "SkeletalMeshComponent Object Reference") (Animation :type "AnimSequenceBase Object Reference"))
  (returns (ReturnValue :type Boolean))
  (locals (`L CombatCharacter` :type "/Game/DynamicCombatSystem/Blueprints/BP_CombatCharacter Object Reference"))
  (bind _returnvalue (`ActorComponent.GetOwner` MeshComp))
  (bind _l_combatcharacter (`local.L CombatCharacter`))
  (bind _bowarrow (`/Game/DynamicCombatSystem/Blueprints/BP_CombatCharacter.BowArrow` _l_combatcharacter))
  (`/Engine/EditorBlueprintResources/StandardMacros.IsValid` _returnvalue
    (:`Is Valid`
      (bind _asbp_combat_character (cast `/Game/DynamicCombatSystem/Blueprints/BP_CombatCharacter` _returnvalue))
      (set `local.L CombatCharacter` _asbp_combat_character)
      (if (`self.AttachToHand`)
        (bind _name (message `/Game/DynamicCombatSystem/Blueprints/Interfaces/I_IsArcher.GetBowStringSocketName` _l_combatcharacter))
        (`SceneComponent.K2_AttachToComponent` _bowarrow (`Character.Mesh` (`local.L CombatCharacter`)) _name "SnapToTarget" "SnapToTarget" "SnapToTarget" false)
        (else
          (`SceneComponent.K2_AttachToComponent` _bowarrow (`/Game/DynamicCombatSystem/Blueprints/BP_CombatCharacter.BowMesh` (`local.L CombatCharacter`)) "arrow" "SnapToTarget" "SnapToTarget" "SnapToTarget" false)))
      (`SceneComponent.SetVisibility` (`/Game/DynamicCombatSystem/Blueprints/BP_CombatCharacter.BowArrow` (`local.L CombatCharacter`)) (`self.ArrowVisibility`) false)
      (return false))))