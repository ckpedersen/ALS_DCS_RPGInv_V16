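; Anim notify that updates the arrow mesh on an archer AI during bow animations.
; It casts the mesh owner to BP_ArcherAI and snaps its BowArrow component either to a character mesh socket, named by GetBowStringSocketNameMessage, or to the arrow socket on the bow mesh, depending on AttachToHand.
; It then sets the arrow's visibility from the ArrowVisibility setting.
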(fn `Received_Notify`
  (params (MeshComp :type "SkeletalMeshComponent Object Reference") (Animation :type "AnimSequenceBase Object Reference"))
  (returns (ReturnValue :type Boolean))
  (locals (`L ArcherAI` :type "/Game/DynamicCombatSystem/Blueprints/AI/Archer/BP_ArcherAI Object Reference"))
  (bind _returnvalue (`ActorComponent.GetOwner` MeshComp))
  (bind _l_archerai (`local.L ArcherAI`))
  (bind _bowarrow (`/Game/DynamicCombatSystem/Blueprints/AI/Archer/BP_ArcherAI.BowArrow` _l_archerai))
  (`/Engine/EditorBlueprintResources/StandardMacros.IsValid` _returnvalue
    (:`Is Valid`
      (bind _asbp_archer_ai (cast `/Game/DynamicCombatSystem/Blueprints/AI/Archer/BP_ArcherAI` _returnvalue))
      (set `local.L ArcherAI` _asbp_archer_ai)
      (if (`self.AttachToHand`)
        (bind _name (message `/Game/DynamicCombatSystem/Blueprints/Interfaces/I_IsArcher.GetBowStringSocketName` _l_archerai))
        (`SceneComponent.K2_AttachToComponent` _bowarrow (`Character.Mesh` (`local.L ArcherAI`)) _name "SnapToTarget" "SnapToTarget" "SnapToTarget" false)
        (else
          (`SceneComponent.K2_AttachToComponent` _bowarrow (`/Game/DynamicCombatSystem/Blueprints/AI/Archer/BP_ArcherAI.BowMesh` (`local.L ArcherAI`)) "arrow" "SnapToTarget" "SnapToTarget" "SnapToTarget" false)))
      (`SceneComponent.SetVisibility` (`/Game/DynamicCombatSystem/Blueprints/AI/Archer/BP_ArcherAI.BowArrow` (`local.L ArcherAI`)) (`self.ArrowVisibility`) false)
      (return false))))