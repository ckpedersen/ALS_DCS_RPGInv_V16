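; Player capture actor for the RPG inventory that mirrors equipped gear on its meshes for a toggleable SceneCapture2D and also runs timed consumable effects.
; Attach/Detach swap meshes by item slot, with armor pieces following the body through master pose.
; Per-stat timelines, rate-scaled by duration, feed rotation values to the ActionConsumables component and remove their assigned effect when finished.
; Drunk and Night Vision effects add post-process components, with Drunk also shaking the player's follow camera.
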(event `Event Start Capture`
  ;[0 1 0.08226 0.227] Start Capture
  (set `SceneCaptureComponent.bCaptureEveryFrame` true (`self.SceneCaptureComponent2D`)))

(event `Event End Capture`
  ;[1 0 0.01016 0.269] End Capture
  (set `SceneCaptureComponent.bCaptureEveryFrame` false (`self.SceneCaptureComponent2D`)))

(event `Play Additional Effect`
  (params (`Additional Effect` :type "/Game/RPG_InventorySystem/ItemsData/Enums/E_AdditionalEffect Enum" :default "NewEnumerator2"))
  ;[0.3168 1 0 0.178] Play Additional Effect
  (switch `/Game/RPG_InventorySystem/ItemsData/Enums/E_AdditionalEffect` `Additional Effect`
    (:`NewEnumerator0`
      ;;[1 0 0.7231 0.217] Effect - Drunk
      (`/Engine/EditorBlueprintResources/StandardMacros.IsValid` (`self.PostProcess Drunk Ref`)
        (:`Is Not Valid`
          (bind _returnvalue (`AddComponent|NODE_AddPostProcessComponent-0`))
          (set `self.PostProcess Drunk Ref` _returnvalue)
          (if (`TimelineComponent.IsPlaying` (`self.CameraShakeTimeline`))
            (bind (_direction _newtrack_0) (`Timeline|CameraShakeTimeline` :!label _label)
              (:`Update`
                (`SceneComponent.K2_SetRelativeTransform` (`/Game/DynamicCombatSystem/Blueprints/BP_CombatCharacter.FollowCamera` (`self.Player Ref`)) (`KismetMathLibrary.MakeTransform` _newtrack_0) false false)))
            (else
              (goto _label :!via `PlayFromStart`))))))
    (:`NewEnumerator1`
      ;;[0.4358 0 1 0.217] Effect - NightVision
      (`/Engine/EditorBlueprintResources/StandardMacros.IsValid` (`self.PostProcess NightVision`)
        (:`Is Not Valid`
          (bind _returnvalue_2 (`AddComponent|NODE_AddPostProcessComponent-1`))
          (set `self.PostProcess NightVision` _returnvalue_2))))))

(event `self.ReceiveBeginPlay`
  ;[0 0.3476 1 0.217] Set References
  (bind _ac_inventory (`/Game/RPG_InventorySystem/Blueprints/BFL_Inventory.Get AC Inventory` :!label _label_2))
  (set `self.Inventory Component` _ac_inventory)
  (`/Game/RPG_InventorySystem/Blueprints/Components/AC_Inventory.Pass Player Capture Reference` (`self.Inventory Component`) self)
  (bind _player (`/Game/RPG_InventorySystem/Blueprints/BFL_Inventory.Get Player Reference`))
  (set `self.Player Ref` _player)
  (bind _returnvalue (`/Game/RPG_InventorySystem/Blueprints/BFL_Inventory.Get AC Action Consumables`))
  (set `self.ActionConsumables Component` _returnvalue))

(event `Event Initialize Timeline`
  (params (Duration :type "Float (double-precision)") (Stat :type "/Game/RPG_InventorySystem/ItemsData/Enums/E_StatCategory Enum" :default "NewEnumerator8") (`Additional Effect` :type "/Game/RPG_InventorySystem/ItemsData/Enums/E_AdditionalEffect Enum" :default "NewEnumerator2"))
  (bind _additional_effect (`self.Additional Effect`))
  (bind _additional_effect_2 (`self.Additional Effect`))
  (bind _additional_effect_3 (`self.Additional Effect`))
  (bind _additional_effect_4 (`self.Additional Effect`))
  (bind _additional_effect_5 (`self.Additional Effect`))
  (bind _additional_effect_6 (`self.Additional Effect`))
  (bind _additional_effect_7 (`self.Additional Effect`))
  ;[0.4553 0.427 1 0.091] Initialize Effect Timeline
  (set `self.Timeline Duration` (/ 1.0 Duration))
  (set `self.Additional Effect` `Additional Effect`)
  (switch `/Game/RPG_InventorySystem/ItemsData/Enums/E_StatCategory` Stat
    (:`NewEnumerator0`
      ;[0 1 0.1711 0.227 24] Health
      (`self.Clear AdditionalEffect from Stat` "NewEnumerator0")
      (`self.Assign Additional Effect` "NewEnumerator0" _additional_effect)
      (`self.Play Additional Effect` _additional_effect)
      (`TimelineComponent.SetPlayRate` (`self.HealthTimeline`) (`self.Timeline Duration`))
      (bind (_direction _value) (`Timeline|HealthTimeline` :!via `PlayFromStart`)
        (:`Update`
          (set `/Game/RPG_InventorySystem/Blueprints/Components/AC_ActionConsumables.HealthRotationValue` _value (`self.ActionConsumables Component`)))
        (:`Finished`
          (`self.Remove Additional Effect` (`self.HealthAdditionalEffect`)))))
    (:`NewEnumerator6`
      ;[0 1 0.4581 0.227 24] MaxHealth
      (`self.Clear AdditionalEffect from Stat` "NewEnumerator6")
      (`self.Assign Additional Effect` "NewEnumerator6" _additional_effect_4)
      (`self.Play Additional Effect` _additional_effect_4)
      (`TimelineComponent.SetPlayRate` (`self.MaxHealthTimeline`) (`self.Timeline Duration`))
      (bind (_direction_2 _value_2) (`Timeline|MaxHealthTimeline` :!via `PlayFromStart`)
        (:`Update`
          (set `/Game/RPG_InventorySystem/Blueprints/Components/AC_ActionConsumables.MaxHealthRotationValue` _value_2 (`self.ActionConsumables Component`)))
        (:`Finished`
          (`self.Remove Additional Effect` (`self.MaxHealthAdditionalEffect`)))))
    (:`NewEnumerator1`
      ;[0.9699 1 0 0.227 24] Stamina
      (`self.Clear AdditionalEffect from Stat` "NewEnumerator1")
      (`self.Assign Additional Effect` "NewEnumerator1" _additional_effect_5)
      (`self.Play Additional Effect` _additional_effect_5)
      (`TimelineComponent.SetPlayRate` (`self.StaminaTimeline`) (`self.Timeline Duration`))
      (bind (_direction_3 _value_3) (`Timeline|StaminaTimeline` :!via `PlayFromStart`)
        (:`Update`
          (set `/Game/RPG_InventorySystem/Blueprints/Components/AC_ActionConsumables.StaminaRotationValue` _value_3 (`self.ActionConsumables Component`)))
        (:`Finished`
          (`self.Remove Additional Effect` (`self.StaminaAdditionalEffect`)))))
    (:`NewEnumerator7`
      ;[0.7706 1 0 0.227 24] MaxStamina
      (`self.Clear AdditionalEffect from Stat` "NewEnumerator7")
      (`self.Assign Additional Effect` "NewEnumerator7" _additional_effect_6)
      (`self.Play Additional Effect` _additional_effect_6)
      (`TimelineComponent.SetPlayRate` (`self.MaxStaminaTimeline`) (`self.Timeline Duration`))
      (bind (_direction_4 _value_4) (`Timeline|MaxStaminaTimeline` :!via `PlayFromStart`)
        (:`Update`
          (set `/Game/RPG_InventorySystem/Blueprints/Components/AC_ActionConsumables.MaxStaminaRotationValue` _value_4 (`self.ActionConsumables Component`)))
        (:`Finished`
          (`self.Remove Additional Effect` (`self.MaxStaminaAdditionalEffect`)))))
    (:`NewEnumerator2`
      ;[1 0.5944 0 0.227 24] Armor
      (`self.Clear AdditionalEffect from Stat` "NewEnumerator2")
      (`self.Assign Additional Effect` "NewEnumerator2" _additional_effect_7)
      (`self.Play Additional Effect` _additional_effect_7)
      (`TimelineComponent.SetPlayRate` (`self.ArmorTimeline`) (`self.Timeline Duration`))
      (bind (_direction_5 _value_5) (`Timeline|ArmorTimeline` :!via `PlayFromStart`)
        (:`Update`
          (set `/Game/RPG_InventorySystem/Blueprints/Components/AC_ActionConsumables.ArmorRotationValue` _value_5 (`self.ActionConsumables Component`)))
        (:`Finished`
          (`self.Remove Additional Effect` (`self.ArmorAdditionalEffect`)))))
    (:`NewEnumerator3`
      ;[1 0 0.01469 0.227 24] Damage
      (`self.Clear AdditionalEffect from Stat` "NewEnumerator3")
      (`self.Assign Additional Effect` "NewEnumerator3" _additional_effect_2)
      (`self.Play Additional Effect` _additional_effect_2)
      (`TimelineComponent.SetPlayRate` (`self.DamageTimeline`) (`self.Timeline Duration`))
      (bind (_direction_6 _value_6) (`Timeline|DamageTimeline` :!via `PlayFromStart`)
        (:`Update`
          (set `/Game/RPG_InventorySystem/Blueprints/Components/AC_ActionConsumables.DamageRotationValue` _value_6 (`self.ActionConsumables Component`)))
        (:`Finished`
          (`self.Remove Additional Effect` (`self.DamageAdditionalEffect`)))))
    (:`NewEnumerator4`
      ;[1 0 0.1175 0.227 24] Attack Speed
      (`self.Clear AdditionalEffect from Stat` "NewEnumerator4")
      (`self.Assign Additional Effect` "NewEnumerator4" _additional_effect_3)
      (`self.Play Additional Effect` _additional_effect_3)
      (`TimelineComponent.SetPlayRate` (`self.AttackSpeedTimeline`) (`self.Timeline Duration`))
      (bind (_direction_7 _value_7) (`Timeline|AttackSpeedTimeline` :!via `PlayFromStart`)
        (:`Update`
          (set `/Game/RPG_InventorySystem/Blueprints/Components/AC_ActionConsumables.AttackSpeedRotationValue` _value_7 (`self.ActionConsumables Component`)))
        (:`Finished`
          (`self.Remove Additional Effect` (`self.AttackSpeedAdditionalEffect`)))))))

(event `Initialize Player Capture`
  ;[0 0.3476 1 0.217] Set References
  (goto _label_2))

(event `Remove Additional Effect`
  (params (`Additional Effect` :type "/Game/RPG_InventorySystem/ItemsData/Enums/E_AdditionalEffect Enum" :default "NewEnumerator2"))
  (bind _postprocess_drunk_ref (`self.PostProcess Drunk Ref`))
  (bind _postprocess_nightvision (`self.PostProcess NightVision`))
  ;[1 0 0.1103 0.157] Remove Additional Effect
  (switch `/Game/RPG_InventorySystem/ItemsData/Enums/E_AdditionalEffect` `Additional Effect`
    (:`NewEnumerator0`
      ;;[1 0 0.7231 0.217] Effect - Drunk
      (`TimelineComponent.Stop` (`self.CameraShakeTimeline`))
      (`/Engine/EditorBlueprintResources/StandardMacros.IsValid` _postprocess_drunk_ref
        (:`Is Valid`
          (`ActorComponent.K2_DestroyComponent` _postprocess_drunk_ref))
        (:`Is Not Valid`
          _))
      (`KismetSystemLibrary.MoveComponentTo` (`/Game/DynamicCombatSystem/Blueprints/BP_CombatCharacter.FollowCamera` (`self.Player Ref`)) (0.0 0.0 0.0) (struct) false false 0.5))
    (:`NewEnumerator1`
      ;;[0.4358 0 1 0.217] Effect - NightVision
      (`/Engine/EditorBlueprintResources/StandardMacros.IsValid` _postprocess_nightvision
        (:`Is Valid`
          (`ActorComponent.K2_DestroyComponent` _postprocess_nightvision))))))

(event `Stop Timeline`
  ;[0.4167 0.01544 0 0.347] Play/Stop Timelines
  (`TimelineComponent.Stop` (`self.HealthTimeline`))
  (`TimelineComponent.Stop` (`self.StaminaTimeline`))
  (`TimelineComponent.Stop` (`self.ArmorTimeline`))
  (`TimelineComponent.Stop` (`self.DamageTimeline`))
  (`TimelineComponent.Stop` (`self.AttackSpeedTimeline`))
  (`TimelineComponent.Stop` (`self.MaxHealthTimeline`))
  (`TimelineComponent.Stop` (`self.MaxStaminaTimeline`)))

(event `Play Timeline`
  ;[0.4167 0.01544 0 0.347] Play/Stop Timelines
  (`TimelineComponent.Play` (`self.HealthTimeline`))
  (`TimelineComponent.Play` (`self.StaminaTimeline`))
  (`TimelineComponent.Play` (`self.ArmorTimeline`))
  (`TimelineComponent.Play` (`self.DamageTimeline`))
  (`TimelineComponent.Play` (`self.AttackSpeedTimeline`))
  (`TimelineComponent.Play` (`self.MaxHealthTimeline`))
  (`TimelineComponent.Play` (`self.MaxStaminaTimeline`)))

(event `Event Attach to Player Capture`
  (params (`Item Data` :type "/Game/RPG_InventorySystem/ItemsData/Structs/S_ItemData Structure"))
  ;[0.05725 1 0 0.248] Attach Item
  (`self.Attach Item` `Item Data`))

(event `Event Detach from Player Capture`
  (params (`Item Data` :type "/Game/RPG_InventorySystem/ItemsData/Structs/S_ItemData Structure"))
  ;[1 0.02893 0 0.243] Detach Item
  (`self.Detach Item` `Item Data`))

(fn `Assign Additional Effect`
  (params (Stat :type "/Game/RPG_InventorySystem/ItemsData/Enums/E_StatCategory Enum" :default "NewEnumerator8") (AdditionalEffect :type "/Game/RPG_InventorySystem/ItemsData/Enums/E_AdditionalEffect Enum" :default "NewEnumerator2"))
  (switch `/Game/RPG_InventorySystem/ItemsData/Enums/E_StatCategory` Stat
    (:`NewEnumerator0`
      (set `self.HealthAdditionalEffect` AdditionalEffect))
    (:`NewEnumerator6`
      (set `self.MaxHealthAdditionalEffect` AdditionalEffect))
    (:`NewEnumerator1`
      (set `self.StaminaAdditionalEffect` AdditionalEffect))
    (:`NewEnumerator7`
      (set `self.MaxStaminaAdditionalEffect` AdditionalEffect))
    (:`NewEnumerator2`
      (set `self.ArmorAdditionalEffect` AdditionalEffect))
    (:`NewEnumerator3`
      (set `self.DamageAdditionalEffect` AdditionalEffect))
    (:`NewEnumerator4`
      (set `self.AttackSpeedAdditionalEffect` AdditionalEffect))))

(fn `Attach Item`
  (params (`Item Data` :type "/Game/RPG_InventorySystem/ItemsData/Structs/S_ItemData Structure"))
  (locals (ItemClass :type "/Game/RPG_InventorySystem/ItemClasses/Interactable/BP_BASE_ITEM Class Reference") (`L Item Slot` :type "/Game/RPG_InventorySystem/ItemsData/Enums/E_ItemSlot Enum") (`L Static Mesh` :type "StaticMesh Object Reference") (`L Skeletal Mesh` :type "SkeletalMesh Object Reference"))
  (bind ((`Slot_34_D8E166834B91EEF8631726AE76BDFFE0` _slot) (`EquippableStaticMesh_58_499FB0724FB11A097DFBFE96CE732928` _equippablestaticmesh) (`EquippableSkeletalMesh_59_B73DB7FB4045D2047189D4927239E34B` _equippableskeletalmesh)) (break `/Game/RPG_InventorySystem/ItemsData/Structs/S_ItemData` `Item Data`))
  (bind _l_static_mesh (`local.L Static Mesh`))
  (bind _l_skeletal_mesh (`local.L Skeletal Mesh`))
  (bind _l_skeletal_mesh_2 (`local.L Skeletal Mesh`))
  (bind _l_static_mesh_2 (`local.L Static Mesh`))
  (bind _returnvalue (select `/Game/RPG_InventorySystem/ItemsData/Enums/E_ItemSlot` (`local.L Item Slot`) :`NewEnumerator1` (`self.Head`) :`NewEnumerator2` (`self.Gloves`) :`NewEnumerator4` (`self.Chestplate`) :`NewEnumerator5` (`self.Legs`) :`NewEnumerator6` (`self.Boots`)))
  (set `local.L Item Slot` _slot)
  (set `local.L Static Mesh` _equippablestaticmesh)
  (set `local.L Skeletal Mesh` _equippableskeletalmesh)
  (switch `/Game/RPG_InventorySystem/ItemsData/Enums/E_ItemSlot` (`local.L Item Slot`)
    (:`NewEnumerator1`
      ;[0.05725 1 0 0.285 22] Attach Armor [Skeletal]
      (`/Engine/EditorBlueprintResources/StandardMacros.IsValid` _returnvalue :!label _label
        (:`Is Valid`
          (`/Engine/EditorBlueprintResources/StandardMacros.IsValid` _l_skeletal_mesh_2
            (:`Is Valid`
              (`SkinnedMeshComponent.SetSkinnedAssetAndUpdate` _returnvalue _l_skeletal_mesh_2 true)
              (`SkinnedMeshComponent.SetLeaderPoseComponent` _returnvalue (`self.SkeletalMesh`) false))))))
    (:`NewEnumerator2`
      (goto _label))
    (:`NewEnumerator4`
      (goto _label))
    (:`NewEnumerator5`
      (goto _label))
    (:`NewEnumerator6`
      (goto _label))
    (:`NewEnumerator7`
      ;[1 0.5216 0 0.243 22] Attach Weapon [Static]
      (`/Engine/EditorBlueprintResources/StandardMacros.IsValid` _l_static_mesh_2
        (:`Is Valid`
          (`StaticMeshComponent.SetStaticMesh` (`self.Weapon`) _l_static_mesh_2))))
    (:`NewEnumerator12`
      ;[1 0.02652 0 0.243 22] Attach Shield [Static]
      (`/Engine/EditorBlueprintResources/StandardMacros.IsValid` _l_static_mesh
        (:`Is Valid`
          (`StaticMeshComponent.SetStaticMesh` (`self.Shield`) _l_static_mesh))))
    (:`NewEnumerator13`
      ;[0 0.4822 1 0.243 22] Bow
      (`/Engine/EditorBlueprintResources/StandardMacros.IsValid` _l_skeletal_mesh
        (:`Is Valid`
          (`SkinnedMeshComponent.SetSkinnedAssetAndUpdate` (`self.Bow`) _l_skeletal_mesh true))))))

(fn `Clear AdditionalEffect from Stat`
  (params (Stat :type "/Game/RPG_InventorySystem/ItemsData/Enums/E_StatCategory Enum" :default "NewEnumerator8"))
  (bind _returnvalue (select `/Game/RPG_InventorySystem/ItemsData/Enums/E_StatCategory` Stat :`NewEnumerator8` "NewEnumerator2" :`NewEnumerator0` (`self.HealthAdditionalEffect`) :`NewEnumerator6` (`self.MaxHealthAdditionalEffect`) :`NewEnumerator1` (`self.StaminaAdditionalEffect`) :`NewEnumerator7` (`self.MaxStaminaAdditionalEffect`) :`NewEnumerator2` (`self.ArmorAdditionalEffect`) :`NewEnumerator3` (`self.DamageAdditionalEffect`) :`NewEnumerator4` (`self.AttackSpeedAdditionalEffect`)))
  (if (not (`|EnumEquality` _returnvalue "NewEnumerator2"))
    (`self.Remove Additional Effect` _returnvalue)
    (`self.Assign Additional Effect` Stat)))

(fn `Detach Item`
  (params (`Item Data` :type "/Game/RPG_InventorySystem/ItemsData/Structs/S_ItemData Structure"))
  (locals (`L Item Slot` :type "/Game/RPG_InventorySystem/ItemsData/Enums/E_ItemSlot Enum"))
  (bind _bow (`self.Bow`))
  (bind _weapon (`self.Weapon`))
  (bind _shield (`self.Shield`))
  (bind _returnvalue (select `/Game/RPG_InventorySystem/ItemsData/Enums/E_ItemSlot` (`local.L Item Slot`) :`NewEnumerator1` (`self.Head`) :`NewEnumerator2` (`self.Gloves`) :`NewEnumerator4` (`self.Chestplate`) :`NewEnumerator5` (`self.Legs`) :`NewEnumerator6` (`self.Boots`) :!type "SkinnedMeshComponent Object Reference"))
  (bind _output_get (set `local.L Item Slot` (`.Slot_34_D8E166834B91EEF8631726AE76BDFFE0` (break `/Game/RPG_InventorySystem/ItemsData/Structs/S_ItemData` `Item Data`))))
  (switch `/Game/RPG_InventorySystem/ItemsData/Enums/E_ItemSlot` _output_get
    (:`NewEnumerator1`
      ;[0.05725 1 0 0.285 22] Detach Armor [Skeletal]
      (`/Engine/EditorBlueprintResources/StandardMacros.IsValid` _returnvalue :!label _label
        (:`Is Valid`
          (`SkinnedMeshComponent.SetSkinnedAssetAndUpdate` _returnvalue null true))))
    (:`NewEnumerator2`
      (goto _label))
    (:`NewEnumerator4`
      (goto _label))
    (:`NewEnumerator5`
      (goto _label))
    (:`NewEnumerator6`
      (goto _label))
    (:`NewEnumerator7`
      ;[1 0.5216 0 0.243 22] Detach Weapon [Static]
      (`/Engine/EditorBlueprintResources/StandardMacros.IsValid` _weapon
        (:`Is Valid`
          (`StaticMeshComponent.SetStaticMesh` _weapon null))))
    (:`NewEnumerator12`
      ;[1 0.02652 0 0.243 22] Detach Shield [Static]
      (`/Engine/EditorBlueprintResources/StandardMacros.IsValid` _shield
        (:`Is Valid`
          (`StaticMeshComponent.SetStaticMesh` _shield null))))
    (:`NewEnumerator13`
      ;[0 0.7302 1 0.243 22] Bow
      (`/Engine/EditorBlueprintResources/StandardMacros.IsValid` _bow
        (:`Is Valid`
          (`SkinnedMeshComponent.SetSkinnedAssetAndUpdate` _bow null true))))))

(fn `Is assigned to other stat?`
  (params (Stat :type "/Game/RPG_InventorySystem/ItemsData/Enums/E_StatCategory Enum" :default "NewEnumerator8"))
  (returns (`Is?` :type Boolean))
  (bind _returnvalue (select `/Game/RPG_InventorySystem/ItemsData/Enums/E_StatCategory` Stat :`NewEnumerator8` "NewEnumerator2" :`NewEnumerator0` (`self.HealthAdditionalEffect`) :`NewEnumerator6` (`self.MaxHealthAdditionalEffect`) :`NewEnumerator1` (`self.StaminaAdditionalEffect`) :`NewEnumerator7` (`self.MaxStaminaAdditionalEffect`) :`NewEnumerator2` (`self.ArmorAdditionalEffect`) :`NewEnumerator3` (`self.DamageAdditionalEffect`) :`NewEnumerator4` (`self.AttackSpeedAdditionalEffect`)))
  (if (> (+ (`KismetMathLibrary.Conv_BoolToInt` (`|EnumEquality` _returnvalue (`self.HealthAdditionalEffect`))) (`KismetMathLibrary.Conv_BoolToInt` (`|EnumEquality` _returnvalue (`self.StaminaAdditionalEffect`))) (`KismetMathLibrary.Conv_BoolToInt` (`|EnumEquality` _returnvalue (`self.ArmorAdditionalEffect`))) (`KismetMathLibrary.Conv_BoolToInt` (`|EnumEquality` _returnvalue (`self.DamageAdditionalEffect`))) (`KismetMathLibrary.Conv_BoolToInt` (`|EnumEquality` _returnvalue (`self.AttackSpeedAdditionalEffect`))) (`KismetMathLibrary.Conv_BoolToInt` (`|EnumEquality` _returnvalue (`self.MaxHealthAdditionalEffect`))) (`KismetMathLibrary.Conv_BoolToInt` (`|EnumEquality` _returnvalue (`self.MaxStaminaAdditionalEffect`)))) 1)
    (return true)
    (else
      (return false))))

(fn `UserConstructionScript`)