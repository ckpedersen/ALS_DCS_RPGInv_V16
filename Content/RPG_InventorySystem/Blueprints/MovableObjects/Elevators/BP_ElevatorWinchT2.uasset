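; BP_ElevatorWinchT2 is an elevator winch whose mesh rotates and whose rope attaches to a linked MovableObject.
; On BeginPlay it binds to that object's AC_MovableObject move, reverse, stop and finish events.
; A timeline drives the mesh's roll, with separate handlers playing it forward, reversing it or stopping it.
; The construction script attaches the rope's end to the linked object's CableEnd2 component.
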(event `self.ReceiveBeginPlay`
  (bind _movable_object (`self.Movable Object`))
  (bind _returnvalue (`self.GetComponentByClass` _movable_object "/Game/RPG_InventorySystem/Blueprints/Components/AC_MovableObject.AC_MovableObject_C"))
  (`/Engine/EditorBlueprintResources/StandardMacros.IsValid` _movable_object
    (:`Is Valid`
      (`/Engine/EditorBlueprintResources/StandardMacros.IsValid` _returnvalue
        (:`Is Valid`
          (add `/Game/RPG_InventorySystem/Blueprints/Components/AC_MovableObject.On Move` _returnvalue (`|CreateDelegate` :!event `ReverseRotate`))
          (add `/Game/RPG_InventorySystem/Blueprints/Components/AC_MovableObject.On Reverse` _returnvalue (`|CreateDelegate` :!event `PlayRotate`))
          (add `/Game/RPG_InventorySystem/Blueprints/Components/AC_MovableObject.On Stop` _returnvalue (`|CreateDelegate` :!event `StopRotate`))
          (add `/Game/RPG_InventorySystem/Blueprints/Components/AC_MovableObject.On Finished` _returnvalue (`|CreateDelegate` :!event `FinishRotate`)))))))

(event `ReverseRotate`
  (bind (_direction _rotationx) (`Timeline|Timeline_Rotation` :!label _label)
    (:`Update`
      (`SceneComponent.K2_SetRelativeRotation` (`self.StaticMesh`) (`KismetMathLibrary.MakeRotator` (.x _rotationx)) false false))))

(event `StopRotate`
  (goto _label :!via `Stop`))

(event `FinishRotate`
  (goto _label :!via `Stop`))

(event `PlayRotate`
  (goto _label :!via `Reverse`))

(fn `UserConstructionScript`
  (bind _movable_object (`self.Movable Object`))
  (`/Engine/EditorBlueprintResources/StandardMacros.IsValid` _movable_object
    (:`Is Valid`
      (`CableComponent.SetAttachEndTo` (`self.Rope`) _movable_object "CableEnd2" "None"))))