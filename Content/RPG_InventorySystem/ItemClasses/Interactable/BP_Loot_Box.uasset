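; BP_Loot_Box is an interactable loot chest for the RPG inventory system that opens and closes as interaction starts and ends.
; Interaction plays the open animation on the skeletal mesh and hides the ACInteractable component's interaction widget.
; EndInteraction plays the close animation, then shows the widget again after a zero-length delay.
; The construction script only calls its parent, and this Blueprint's graphs contain no loot logic.
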(event `/Game/RPG_InventorySystem/Blueprints/BPI_Interactable.Interaction`
  ;[1 0 0.01436 0.248] Open / Close Chest
  (`SkeletalMeshComponent.PlayAnimation` (`self.SkeletalMesh`) "/Game/RPG_InventorySystem/Animations/Chest_Open.Chest_Open" false)
  ;[0.2775 0 1 0.305] Toggle Interaction Widget
  (`/Game/RPG_InventorySystem/Blueprints/Components/AC_Interactable.Toggle Interaction Widget` (`self.AC_Interactable`) false))

(event `/Game/RPG_InventorySystem/Blueprints/BPI_Interactable.End Interaction`
  ;[1 0 0.01436 0.248] Open / Close Chest
  (`SkeletalMeshComponent.PlayAnimation` (`self.SkeletalMesh`) "/Game/RPG_InventorySystem/Animations/Chest_Close.Chest_Close" false)
  ;[0.2775 0 1 0.305] Toggle Interaction Widget
  (`KismetSystemLibrary.Delay` 0.0)
  (`/Game/RPG_InventorySystem/Blueprints/Components/AC_Interactable.Toggle Interaction Widget` (`self.AC_Interactable`) true))

(fn `UserConstructionScript`
  (`parent.UserConstructionScript`))