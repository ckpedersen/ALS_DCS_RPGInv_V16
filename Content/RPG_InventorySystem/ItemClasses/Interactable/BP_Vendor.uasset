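; BP_Vendor is an interactable vendor actor in the RPG inventory system that randomizes its hair texture on BeginPlay.
; It creates a dynamic hair material instance on skeletal mesh element 14 and also assigns it to element 0.
; A random entry from the first three HairTex textures becomes that material's base color map.
; The construction script only calls its parent, and no vendor logic is defined here.
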(event `self.ReceiveBeginPlay`
  (bind _skeletalmesh (`self.SkeletalMesh`))
  (bind _returnvalue (`PrimitiveComponent.CreateDynamicMaterialInstance` _skeletalmesh 14 "/Game/Characters/Player/Female_HQ_02/Materials/Base_HQ/High_polytail_LWHQ_Inst.High_polytail_LWHQ_Inst" "None"))
  (bind _output_get (set `self.Hair_Mat` _returnvalue))
  (`PrimitiveComponent.SetMaterial` _skeletalmesh 0 _output_get)
  (`MaterialInstanceDynamic.SetTextureParameterValue` (`self.Hair_Mat`) "Base Color Map" (`|GetArrayItem` (`self.Hair_Tex`) (`KismetMathLibrary.RandomIntegerInRange` 0 2))))

(fn `UserConstructionScript`
  (`parent.UserConstructionScript`))